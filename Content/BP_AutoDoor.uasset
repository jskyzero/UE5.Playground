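; BP_AutoDoor is a door that slides open when something overlaps its Area component and closes when an overlap ends.
; BeginPlay stores the Door's relative location as the closed position.
; The DoorLerp timeline plays or reverses on overlap events, feeding its Alpha to MoveDoor, which interpolates between that position and OpenLoaction.
; Overlaps are not filtered by actor or counted.
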(event `self.ReceiveBeginPlay`
  (set `self.InitialLocation` (`SceneComponent.RelativeLocation` (`self.Door`))))

(event `self.Area.OnComponentBeginOverlap`
  (params (OverlappedComponent :type "PrimitiveComponent Object Reference") (OtherActor :type "Actor Object Reference") (OtherComp :type "PrimitiveComponent Object Reference") (OtherBodyIndex :type Integer) (bFromSweep :type Boolean) (SweepResult :type "HitResult Structure (by ref)"))
  (bind (_direction _alpha) (`Timeline|DoorLerp` :!label _label)
    (:`Update`
      (`self.MoveDoor` _alpha))))

(event `self.Area.OnComponentEndOverlap`
  (params (OverlappedComponent :type "PrimitiveComponent Object Reference") (OtherActor :type "Actor Object Reference") (OtherComp :type "PrimitiveComponent Object Reference") (OtherBodyIndex :type Integer))
  (goto _label :!via `Reverse`))

(fn `MoveDoor`
  (params (LerpAlpha :type "Float (double-precision)"))
  (`SceneComponent.K2_SetRelativeLocation` (`self.Door`) (`KismetMathLibrary.VLerp` (`self.InitialLocation`) (`self.OpenLoaction`) LerpAlpha) false false))

(fn `UserConstructionScript`)